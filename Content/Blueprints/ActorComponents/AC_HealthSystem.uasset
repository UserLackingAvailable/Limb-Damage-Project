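; Actor component that tracks total and per-limb health for BP_ThirdPersonCharacter.
; Point damage lowers total health and the limb identified by the hit's physical material surface type, then updates the character's WB_HealthBar widget.
; Zero total health or a destroyed head calls OnDeath, while broken arms trigger events on the owning character.
; Torso and legs have health bars but no break effects.
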(event Custom|Event%20Any%20Point%20Damage
  (params (Damage :type Float%20%28double-precision%29) (Hit :type Hit%20Result%20Structure))
  (bind _physmat (Collision|BreakHitResult Hit))
  (bind _surfacetype (Variables|/Script/PhysicsCore.PhysicalMaterial|GetSurfaceType _physmat))
  (CallFunction|UpdateTotalHealth Damage)
  (bind _remaining_limb_health (CallFunction|UpdateLimbHealth _surfacetype Damage))
  (CallFunction|EventAnyLimbDamage _surfacetype _remaining_limb_health)
  (Development|PrintString (Utilities|String|Append (Utilities|String|EnumtoString _surfacetype) ": " (Utilities|String|ToString(Float) _remaining_limb_health)) true true "(R=0.196938,G=1.000000,B=0.044161,A=1.000000)"))

(event EventBeginPlay)

(event EventTick
  (params (DeltaSeconds :type Float%20%28single-precision%29)))

(fn UpdateTotalHealth
  (params (Damage :type Float%20%28double-precision%29))
  (bind _output_get (Variables|Default|SetTotalHealth (Math|Float|Clamp(Float) (- (Variables|Default|GetTotalHealth) Damage) 0.0 1e+02)))
  (bind _asbp_third_person_character (Utilities|Casting|CastToBP_ThirdPersonCharacter (Components|GetOwner)))
  (bind _aswb_health_bar (Utilities|Casting|CastToWB_HealthBar (UserInterface|GetWidget (Variables|/Game/ThirdPerson/Blueprints/BP_ThirdPersonCharacter.BP_ThirdPersonCharacter_C|GetHealthBarWidget _asbp_third_person_character))))
  (Progress|SetPercent (Variables|/Game/Blueprints/ActorComponents/WB_HealthBar.WB_HealthBar_C|GetHealthBar_Total _aswb_health_bar) (/ _output_get 1e+02))
  (if (<= _output_get 0.0)
    (Default|CallOnDeath))
  (return _output_get))

(fn UpdateLimbHealth
  (params (DamagedLimb :type EPhysicalSurface%20Enum :default "SurfaceType_Default") (Damage :type Float%20%28double-precision%29))
  (Utilities|Map|Add (Variables|Default|GetLimbHealth) DamagedLimb (Math|Float|Truncate (Math|Float|Clamp(Float) (- (.Value (Utilities|Map|Find (Variables|Default|GetLimbHealth) DamagedLimb)) Damage) 0.0 1e+02)))
  (Utilities|FlowControl|Sequence
    (:then_0
      (return (Math|Conversions|ToFloat(Integer) (.Value (Utilities|Map|Find (Variables|Default|GetLimbHealth) DamagedLimb)))))))

(fn EventAnyLimbDamage
  (params (DamagedLimb :type EPhysicalSurface%20Enum :default "SurfaceType_Default") (RemainingLimbHealth :type Float%20%28double-precision%29))
  (bind _returnvalue (<= RemainingLimbHealth 0.0))
  (Utilities|FlowControl|Sequence
    (:then_0
      (switch Utilities|FlowControl|Switch|SwitchonEPhysicalSurface DamagedLimb
        (:SurfaceType1
          ;[0.15 0.15 0.15 0.5] <= 0 Limb Results
          ;;[0.15 0.15 0.15 0.5] Head
          (if _returnvalue
            (bind _remainingtotalhealth (CallFunction|UpdateTotalHealth (Variables|Default|GetTotalHealth)))
            (bind _asbp_third_person_character (Utilities|Casting|CastToBP_ThirdPersonCharacter (Game|Player|GetPlayerPawn 0)))
            (bind _aswb_health_bar (Utilities|Casting|CastToWB_HealthBar (UserInterface|GetWidget (Variables|/Game/ThirdPerson/Blueprints/BP_ThirdPersonCharacter.BP_ThirdPersonCharacter_C|GetHealthBarWidget _asbp_third_person_character))))
            (Progress|SetPercent (Variables|/Game/Blueprints/ActorComponents/WB_HealthBar.WB_HealthBar_C|GetHealthBar_Total _aswb_health_bar) _remainingtotalhealth)
            (Default|CallOnDeath)))
        (:SurfaceType3
          ;;[0.15 0.15 0.15 0.5] Arm_L
          (if _returnvalue
            (Development|PrintString "Left Arm Broken")
            (bind _asbp_third_person_character_2 (Utilities|Casting|CastToBP_ThirdPersonCharacter (Components|GetOwner)))
            (Default|OnLeftArmBroken _asbp_third_person_character_2)))
        (:SurfaceType4
          ;;[0.15 0.15 0.15 0.5] Arm_R
          (if _returnvalue
            (Development|PrintString "Right Arm Broken")
            (bind _asbp_third_person_character_3 (Utilities|Casting|CastToBP_ThirdPersonCharacter (Components|GetOwner)))
            (Default|OnRightArmBroken _asbp_third_person_character_3)))))
    (:then_1
      ;[0.15 0.15 0.15 0.5] Limb Healthbars
      (bind _asbp_third_person_character_4 (Utilities|Casting|CastToBP_ThirdPersonCharacter (Components|GetOwner)))
      (bind _aswb_health_bar_2 (Utilities|Casting|CastToWB_HealthBar (UserInterface|GetWidget (Variables|/Game/ThirdPerson/Blueprints/BP_ThirdPersonCharacter.BP_ThirdPersonCharacter_C|GetHealthBarWidget _asbp_third_person_character_4))))
      (switch Utilities|FlowControl|Switch|SwitchonEPhysicalSurface DamagedLimb
        (:SurfaceType1
          (Progress|SetPercent (Variables|/Game/Blueprints/ActorComponents/WB_HealthBar.WB_HealthBar_C|GetHealthBar_Head _aswb_health_bar_2) (/ RemainingLimbHealth 2e+01)))
        (:SurfaceType2
          (Progress|SetPercent (Variables|/Game/Blueprints/ActorComponents/WB_HealthBar.WB_HealthBar_C|GetHealthBar_Torso _aswb_health_bar_2) (/ RemainingLimbHealth 1e+02)))
        (:SurfaceType3
          (Progress|SetPercent (Variables|/Game/Blueprints/ActorComponents/WB_HealthBar.WB_HealthBar_C|GetHealthBar_ArmL _aswb_health_bar_2) (/ RemainingLimbHealth 4e+01)))
        (:SurfaceType4
          (Progress|SetPercent (Variables|/Game/Blueprints/ActorComponents/WB_HealthBar.WB_HealthBar_C|GetHealthBar_ArmR _aswb_health_bar_2) (/ RemainingLimbHealth 4e+01)))
        (:SurfaceType5
          (Progress|SetPercent (Variables|/Game/Blueprints/ActorComponents/WB_HealthBar.WB_HealthBar_C|GetHealthBar_LegL _aswb_health_bar_2) (/ RemainingLimbHealth 1e+02)))
        (:SurfaceType6
          (Progress|SetPercent (Variables|/Game/Blueprints/ActorComponents/WB_HealthBar.WB_HealthBar_C|GetHealthBar_LegR _aswb_health_bar_2) (/ RemainingLimbHealth 1e+02)))))))